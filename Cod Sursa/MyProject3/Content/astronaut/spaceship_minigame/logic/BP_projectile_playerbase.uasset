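; Base player projectile for the spaceship minigame that damages enemies on hit.
; The construction script applies the configured scale and speed to the mesh and projectile movement and creates a dynamic material, which is tinted blue on BeginPlay.
; Hits on either the projectile component or the box share one handler that applies damage to Enemy_base actors and destroys the projectile whatever it struck.
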(event OnComponentHit(Projectile.)
  (params (HitComponent :type Primitive%20Component%20Object%20Reference) (OtherActor :type Actor%20Object%20Reference) (OtherComp :type Primitive%20Component%20Object%20Reference) (NormalImpulse :type Vector :default "0, 0, 0") (Hit :type Hit%20Result%20Structure%20%28by%20ref%29))
  (bind _asenemy_base (Utilities|Casting|CastToEnemy_base OtherActor)
    (:then
      (Game|Damage|ApplyDamage _asenemy_base (Variables|Default|GetDamage) 0 0))
    (:CastFailed
      _))
  (Actor|DestroyActor))

(event OnComponentHit(Box)
  (params (HitComponent :type Primitive%20Component%20Object%20Reference) (OtherActor :type Actor%20Object%20Reference) (OtherComp :type Primitive%20Component%20Object%20Reference) (NormalImpulse :type Vector :default "0, 0, 0") (Hit :type Hit%20Result%20Structure%20%28by%20ref%29))
  (bind _asenemy_base (Utilities|Casting|CastToEnemy_base (stale OnComponentHit(Projectile.) OtherActor))
    (:then
      (Game|Damage|ApplyDamage _asenemy_base (Variables|Default|GetDamage) 0 0))
    (:CastFailed
      _))
  (Actor|DestroyActor))

(event EventBeginPlay
  (Rendering|Material|SetVectorParameterValue (Variables|Default|GetDyna%20Mat) "Color" "(R=0.000000,G=0.000000,B=1.000000,A=1.000000)" :!class /Script/Engine.MaterialInstanceDynamic))

(event EventTick
  (params (DeltaSeconds :type Float%20%28single-precision%29)))

(fn ConstructionScript
  (bind _projectilemovement (Variables|Default|GetProjectileMovement))
  (bind _projectile_ (Variables|Default|GetProjectile.))
  (bind _returnvalue (Rendering|Material|CreateDynamicMaterialInstance _projectile_ 0 0 "None" :!class /Script/Engine.PrimitiveComponent))
  (Variables|Default|SetDyna%20Mat _returnvalue)
  (Transformation|SetWorldScale3D _projectile_ (Variables|Default|GetScale))
  (bind _output_get (Variables|/Script/Engine.ProjectileMovementComponent|SetMaxSpeed _projectilemovement (Variables|Default|GetSpeed)))
  (Variables|/Script/Engine.ProjectileMovementComponent|SetInitialSpeed _projectilemovement _output_get))