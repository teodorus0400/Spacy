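; Game mode for the spaceship minigame that tracks enemy count, kills and score, and declares a win at 25 kills.
; BeginPlay shows the HUD widget with game-only input, and Tutorial pauses the game behind its own widget.
; EnemyKilled feeds UpdateEnemyCount, which triggers the pawn's win and GameWon screen, while EndPlay triggers its GameOver.
; SaveScore is empty, and LoadScore only adds EnemyValue through SetScore and re-adds the HUD.
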(event Custom|UpdateEnemyCount
  (params (Val :type Integer))
  (Variables|Default|SetEnemyCount (+ (Variables|Default|GetEnemyCount) Val))
  (if (>= (Variables|Default|GetEnemiesKilled) 25)
    (bind _asbp_space_pawn (Utilities|Casting|CastToBP_space_pawn (Game|Player|GetPlayerPawn 0)))
    (Default|GameWon _asbp_space_pawn)
    (Viewport|RemoveAllWidgets)
    (Variables|/Script/Engine.PlayerController|SetbShowMouseCursor (Game|GetPlayerController 0) true)
    (bind _returnvalue (UserInterface|CreateWidget "/Game/astronaut/spaceship_minigame/logic/GameWon.GameWon_C"))
    (UserInterface|Viewport|AddtoViewport _returnvalue 0)))

(event EventBeginPlay
  (bind _returnvalue (Game|GetPlayerController 0))
  (Variables|/Script/Engine.PlayerController|SetbShowMouseCursor _returnvalue false)
  (Input|SetInputModeGameOnly _returnvalue)
  (bind _returnvalue_2 (UserInterface|CreateWidget "/Game/astronaut/spaceship_minigame/logic/WidgetSPC.WidgetSPC_C" _returnvalue))
  (UserInterface|Viewport|AddtoViewport _returnvalue_2 0))

(event EventEndPlay
  (params (EndPlayReason :type EEndPlayReason%20Enum :default "Destroyed"))
  (Viewport|RemoveAllWidgets)
  (bind _asbp_space_pawn (Utilities|Casting|CastToBP_space_pawn (Game|Player|GetPlayerPawn 0)))
  (Default|GameOver _asbp_space_pawn))

(fn ConstructionScript)

(fn SaveScore)

(fn LoadScore
  (CallFunction|SetScore (Variables|Default|GetEnemyValue))
  (bind _returnvalue (UserInterface|CreateWidget "/Game/astronaut/spaceship_minigame/logic/WidgetSPC.WidgetSPC_C" (Game|GetPlayerController 0)))
  (UserInterface|Viewport|AddtoViewport _returnvalue 0))

(fn SetScore
  (params (Val :type Integer))
  (bind _output_get (Variables|Default|SetScore (+ (Variables|Default|GetScore) Val)))
  (if (>= _output_get (Variables|Default|GetTopScore))
    (Variables|Default|SetTopScore _output_get)
    (else
      (Variables|Default|SetTopScore (Variables|Default|GetTopScore)))))

(fn EnemyKilled
  (bind _result (Math|Integer|IncrementInt (Variables|Default|GetEnemiesKilled))
    (:%20%20
      (Variables|Default|SetEnemiesKilled _result)
      (CallFunction|UpdateEnemyCount -1))))

(fn Tutorial
  (Viewport|RemoveAllWidgets)
  (Game|SetGamePaused true)
  (bind _returnvalue (UserInterface|CreateWidget "/Game/astronaut/spaceship_minigame/logic/Tutorial.Tutorial_C" (Game|GetPlayerController 0)))
  (UserInterface|Viewport|AddtoViewport _returnvalue 0))