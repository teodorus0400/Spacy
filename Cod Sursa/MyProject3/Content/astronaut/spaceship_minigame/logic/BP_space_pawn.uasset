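; Player ship pawn for the spaceship minigame, moving along world X and Z.
; A spawn timeline lifts and spins it, then sets MoveEnabled, which gates only firing.
; Interpolated axis input drives swept movement and yaw on Tick, while held fire buttons loop timers spawning single or twin projectiles.
; Lethal damage destroys it with explosion, camera shake and GameOver widget; GameWon removes it and switches input to UI-only.
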(event Custom|SecFire
  (CallFunction|SecondaryFire))

(event Custom|PrimFire
  (CallFunction|PrimaryFire))

(event Custom|GameWon
  (bind _asspc_cont (Utilities|Casting|CastToSPC_Cont (Game|GetPlayerController 0)))
  (Input|SetInputModeUIOnly _asspc_cont 0 "DoNotLock")
  (Actor|DestroyActor))

(event EventBeginPlay
  (bind _asbp_space_gm (Utilities|Casting|CastToBP_space_GM (Game|GetGameMode)))
  (Variables|Default|SetBP_Gamemode _asbp_space_gm)
  (Variables|Default|SetYaw (.Yaw (Math|Rotator|BreakRotator (Transformation|GetActorRotation))))
  (Variables|Default|Setspawn%20location (Transformation|GetActorLocation))
  (bind _speed (Timeline|Spawn%20animation Play)
    (:Update
      (Transformation|SetActorLocation (Math|Vector|Lerp(Vector) (Variables|Default|Getspawn%20location) (+ (Variables|Default|Getspawn%20location) "0, 0,60.000000") _speed) true false)
      (Transformation|SetActorRotation (Math|Rotator|Lerp(Rotator) "0, 0, 0" (Math|Rotator|MakeRotator 0.0 0.0 (Variables|Default|GetSpawnSpin)) _speed)))
    (:Finished
      (Variables|Default|SetMoveEnabled true))))

(event Game|Damage|EventAnyDamage
  (params (Damage :type Float%20%28single-precision%29) (DamageType :type Damage%20Type%20Object%20Reference) (InstigatedBy :type Controller%20Object%20Reference) (DamageCauser :type Actor%20Object%20Reference))
  (bind _output_get (Variables|Default|SetHealth (Math|Float|Clamp(Float) (- (Variables|Default|GetHealth) Damage) 0.0 (Variables|Default|Getmax%20health))))
  (if (<= _output_get 0.0)
    (Actor|DestroyActor)
    (Effects|SpawnEmitteratLocation "/Game/astronaut/MobileStarterContent/Particles/P_Explosion.P_Explosion" "0, 0, 0")
    (Camera|PlayWorldCameraShake "/Game/astronaut/spaceship_minigame/enemies/Shake_S.Shake_S_C" "0, 0, 0" 0.0 1e+04 1.0 true)
    (CallFunction|GameOver)))

(event EventTick
  (params (DeltaSeconds :type Float%20%28single-precision%29))
  (Variables|Default|Setdelta%20seconds DeltaSeconds)
  (Transformation|SetActorLocation (+ (Transformation|GetActorLocation) (Math|Vector|MakeVector (Variables|Default|Gethoz%20speed) 0.0 0.0)) true false)
  (Transformation|SetActorLocation (+ (Transformation|GetActorLocation) (Math|Vector|MakeVector 0.0 0.0 (Variables|Default|Getvert%20speed))) true false)
  (Transformation|SetActorRotation (Math|Interpolation|RInterpTo "0, 0, 0" (Math|Rotator|MakeRotator 0.0 0.0 (+ (.yaw (Transformation|GetActorRotation)) (Variables|Default|Gethoz%20speed))) (Variables|Default|Getdelta%20seconds) 6e+01)))

(event Input|ActionEvents|InputActionSecondaryFire
  (params (Key :type Key%20Structure :default "None"))
  (:Pressed
    (if (Variables|Default|GetMoveEnabled)
      (Utilities|Time|SetTimerbyFunctionName 0 "SecFire" 0.2 true)))
  (:Released
    (Utilities|Time|ClearTimerbyFunctionName 0 "SecFire")))

(event Input|ActionEvents|InputActionPrimaryFire
  (params (Key :type Key%20Structure :default "None"))
  (:Pressed
    (if (Variables|Default|GetMoveEnabled)
      (Utilities|Time|SetTimerbyFunctionName 0 "PrimFire" 0.2 true)))
  (:Released
    (Utilities|Time|ClearTimerbyFunctionName 0 "PrimFire")))

(event Input|AxisEvents|InputAxisMoveRight
  (params (AxisValue :type Float%20%28single-precision%29))
  ;[1 1 1] Movement
  (Variables|Default|Sethoz%20speed (Math|Interpolation|FInterpTo (Variables|Default|Gethoz%20speed) (* AxisValue (Variables|Default|Getmovement%20speed) (Variables|Default|Getdelta%20seconds)) (Variables|Default|Getdelta%20seconds) 6.0)))

(event Input|AxisEvents|InputAxisIncreaseThrottle/MoveForward
  (params (AxisValue :type Float%20%28single-precision%29))
  (bind _delta_seconds (Variables|Default|Getdelta%20seconds))
  ;[1 1 1] Movement
  (Variables|Default|Setvert%20speed (Math|Interpolation|FInterpTo (Variables|Default|Getvert%20speed) (* AxisValue (Variables|Default|Getmovement%20speed) _delta_seconds) _delta_seconds 6.0)))

(fn ConstructionScript
  (Variables|Default|SetHealth (Variables|Default|Getmax%20health)))

(fn PrimaryFire
  (Game|SpawnActorfromClass "/Game/astronaut/spaceship_minigame/logic/BP_projectile_1.BP_projectile_1_C" (Transformation|GetWorldTransform (Variables|Default|GetprojectileSpawner)) "AlwaysSpawn" 0 (LocalVariables|GetProj%20Color) 0)
  (if (not (Variables|Default|Getshooting))
    (Variables|Default|Setshooting true)
    (Audio|PlaySoundatLocation "/Game/astronaut/spaceship_minigame/sounds/Shot.Shot" (Transformation|GetWorldLocation (Variables|Default|GetplayerMesh)) "0, 0, 0" 1.0 1.0 0.0 0 0 0)
    (Variables|Default|Setshooting false)))

(fn SecondaryFire
  (bind _color (LocalVariables|GetColor))
  (Game|SpawnActorfromClass "/Game/astronaut/spaceship_minigame/logic/BP_projectile_2.BP_projectile_2_C" (Transformation|GetWorldTransform (Variables|Default|GetprojectileSpawner1)) "AlwaysSpawn" 0 _color 0)
  (Game|SpawnActorfromClass "/Game/astronaut/spaceship_minigame/logic/BP_projectile_2.BP_projectile_2_C" (Transformation|GetWorldTransform (Variables|Default|GetprojectileSpawner2)) "AlwaysSpawn" 0 _color 0)
  (if (not (Variables|Default|Getshooting))
    (Variables|Default|Setshooting true)
    (Audio|PlaySoundatLocation "/Game/astronaut/spaceship_minigame/sounds/Shot.Shot" (Transformation|GetWorldLocation (Variables|Default|GetplayerMesh)) "0, 0, 0" 1.0 1.0 0.0 0 0 0)
    (Variables|Default|Setshooting false)))

(fn GameOver
  (bind _returnvalue (UserInterface|CreateWidget "/Game/astronaut/spaceship_minigame/logic/GameOver.GameOver_C"))
  (UserInterface|Viewport|AddtoViewport _returnvalue 0)
  (bind _asspc_cont (Utilities|Casting|CastToSPC_Cont (Game|GetPlayerController 0)))
  (Variables|/Script/Engine.PlayerController|SetbShowMouseCursor _asspc_cont true)
  (Input|SetInputModeUIOnly _asspc_cont 0 "DoNotLock"))