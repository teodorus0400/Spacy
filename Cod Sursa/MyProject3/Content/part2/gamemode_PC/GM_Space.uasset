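; GM_Space is the game mode for the space level, handling its start and its win and lose endings.
; BeginPlay shows the Overlay widget, unpauses and hides the cursor for game-only input.
; GameOver and GameWon swap in their 3D end-screen widgets and spawn an explosion, destroying the player's ShipFighter on a loss.
; Both then pause and show the cursor, subject to ship validity checks.
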(event EventBeginPlay
  (Input|SetInputModeGameOnly (Game|GetPlayerController 0))
  (Viewport|RemoveAllWidgets)
  (bind _returnvalue (UserInterface|CreateWidget "/Game/part2/UI/Overlay.Overlay_C" (Game|GetPlayerController 0)))
  (UserInterface|Viewport|AddtoViewport _returnvalue 0)
  (Game|SetGamePaused false)
  (bind _aspc_space (Utilities|Casting|CastToPC_Space (Game|GetPlayerController 0)))
  (Variables|/Script/Engine.PlayerController|SetbShowMouseCursor _aspc_space false))

(event EventTick
  (params (DeltaSeconds :type Float%20%28single-precision%29)))

(fn ConstructionScript)

(fn GameOver
  (bind _returnvalue (Game|Player|GetPlayerPawn 0))
  (bind _asship_fighter (Utilities|Casting|CastToShipFighter _returnvalue))
  (Viewport|RemoveAllWidgets)
  (bind _returnvalue_2 (UserInterface|CreateWidget "/Game/part2/UI/GameOver3D.GameOver3D_C" (Game|GetPlayerController 0)))
  (UserInterface|Viewport|AddtoViewport _returnvalue_2 0)
  (Utilities|IsValid _asship_fighter
    (:Is%20Valid
      (Effects|SpawnEmitteratLocation "/Game/astronaut/MobileStarterContent/Particles/P_Explosion.P_Explosion" (Transformation|GetActorLocation _asship_fighter) "0, 0, 0" "10.000000,10.000000,10.000000")
      (Actor|DestroyActor _asship_fighter)
      (Game|SetGamePaused true)
      (bind _aspc_space (Utilities|Casting|CastToPC_Space (Game|GetPlayerController 0)))
      (Variables|/Script/Engine.PlayerController|SetbShowMouseCursor _aspc_space true))))

(fn GameWon
  (Viewport|RemoveAllWidgets)
  (bind _returnvalue (UserInterface|CreateWidget "/Game/part2/UI/GameWon3D.GameWon3D_C" (Game|GetPlayerController 0)))
  (UserInterface|Viewport|AddtoViewport _returnvalue 0)
  (Utilities|IsValid "/Game/part2/motherShip/MotherShip.MotherShip"
    (:Is%20Valid
      (Effects|SpawnEmitteratLocation "/Game/astronaut/MobileStarterContent/Particles/P_Explosion.P_Explosion" (Transformation|GetActorLocation) "0, 0, 0" "20.000000,20.000000,20.000000")
      (Actor|DestroyActor (LocalVariables|Getspc))
      (Utilities|IsValid "/Game/part2/spaceship_pawn/ShipFighter.ShipFighter"
        (:Is%20Valid
          (Game|SetGamePaused true)
          (bind _aspc_space (Utilities|Casting|CastToPC_Space (Game|GetPlayerController 0)))
          (Variables|/Script/Engine.PlayerController|SetbShowMouseCursor _aspc_space true))))))